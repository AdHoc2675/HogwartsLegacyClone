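; Boss room cutscene trigger that plays LS_BossRoomSequence when something overlaps its box.
; A DoOnce precedes the player cast, so only the first overlap counts, and playback starts only if that actor is a BP_PlayerCharacterBase.
; It spawns two cine cameras, creates the sequence player and binds the player into the sequence before playing.
; The nodes binding the spawned cameras are disconnected and never run.
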(event OnComponentBeginOverlap(Box)
  (params (OverlappedComponent :type Primitive%20Component%20Object%20Reference) (OtherActor :type Actor%20Object%20Reference) (OtherComp :type Primitive%20Component%20Object%20Reference) (OtherBodyIndex :type Integer) (bFromSweep :type Boolean) (SweepResult :type Hit%20Result%20Structure%20%28by%20ref%29))
  (Utilities|FlowControl|DoOnce false
    (:Completed
      (bind _asbp_player_character_base (Utilities|Casting|CastToBP_PlayerCharacterBase OtherActor))
      (Variables|Default|SetPlayer _asbp_player_character_base)
      (bind _returnvalue (Game|SpawnActorfromClass "/Script/CinematicCamera.CineCameraActor" (Math|Transform|MakeTransform "0, 0, 0" "0, 0, 0" "1.000000,1.000000,1.000000") "Undefined" "MultiplyWithRoot" 0 0))
      (Variables|Default|SetCamera1 _returnvalue)
      (bind _returnvalue_2 (Game|SpawnActorfromClass "/Script/CinematicCamera.CineCameraActor" (Math|Transform|MakeTransform "0, 0, 0" "0, 0, 0" "1.000000,1.000000,1.000000") "Undefined" "MultiplyWithRoot" 0 0))
      (Variables|Default|SetCamera2 _returnvalue_2)
      (bind (_outactor _returnvalue_3) (Sequencer|Player|CreateLevelSequencePlayer "/Game/_BP/LevelSequence/LS_BossRoomSequence.LS_BossRoomSequence"))
      (Class|LevelSequenceActor|SetBinding _outactor (|GetSequenceBinding) (Utilities|Array|MakeArray (Variables|Default|GetPlayer)) false)
      (Sequencer|Player|Play _returnvalue_3 :!class /Script/MovieScene.MovieSceneSequencePlayer))))

(fn ConstructionScript)